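; Building component that previews and places cube, cylinder or ramp pieces for the third-person character and opens menu and shop widgets.
; PreviewLoop picks a mesh from the character's Objectindex, line-traces from the follow camera and moves the preview object to the hit.
; E spawns the matching actor at an offset from that location, records it in ThingsToSave and clears BuildMode.
; Tab and B show the menu and shop with UI-only input.
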(event Custom|PreviewLoop
  ;[1 1 1] line trace bs
  (bind _asbp_third_person_character (Utilities|Casting|CastToBP_ThirdPersonCharacter (Game|GetPlayerCharacter 0)))
  (if (== 0 (Variables|/Game/ThirdPerson/Blueprints/BP_ThirdPersonCharacter.BP_ThirdPersonCharacter_C|Getobjectindex _asbp_third_person_character))
    (Variables|/Game/ThirdPerson/Blueprints/BP_ThirdPersonCharacter.BP_ThirdPersonCharacter_C|SetswitchMesh _asbp_third_person_character "/Game/LevelPrototyping/Meshes/SM_Cube.SM_Cube")
    (elif (== 1 (Variables|/Game/ThirdPerson/Blueprints/BP_ThirdPersonCharacter.BP_ThirdPersonCharacter_C|Getobjectindex _asbp_third_person_character))
      (Variables|/Game/ThirdPerson/Blueprints/BP_ThirdPersonCharacter.BP_ThirdPersonCharacter_C|SetswitchMesh _asbp_third_person_character "/Game/LevelPrototyping/Meshes/SM_Cylinder.SM_Cylinder")
      (else
        (Variables|/Game/ThirdPerson/Blueprints/BP_ThirdPersonCharacter.BP_ThirdPersonCharacter_C|SetswitchMesh _asbp_third_person_character "/Game/LevelPrototyping/Meshes/SM_ChamferCube.SM_ChamferCube"))))
  (bind (_outhit _returnvalue) (Collision|LineTraceByChannel (.Location (Math|Transform|BreakTransform (Transformation|GetWorldTransform (Variables|/Game/ThirdPerson/Blueprints/BP_ThirdPersonCharacter.BP_ThirdPersonCharacter_C|GetFollowCamera _asbp_third_person_character)))) (+ (.Location (Math|Transform|BreakTransform (Transformation|GetWorldTransform (Variables|/Game/ThirdPerson/Blueprints/BP_ThirdPersonCharacter.BP_ThirdPersonCharacter_C|GetFollowCamera _asbp_third_person_character)))) (* (Math|Vector|GetForwardVector (.Rotation (Math|Transform|BreakTransform (Transformation|GetWorldTransform (Variables|/Game/ThirdPerson/Blueprints/BP_ThirdPersonCharacter.BP_ThirdPersonCharacter_C|GetFollowCamera _asbp_third_person_character))))) (Math|Conversions|ToVector(Float) 7e+03))) "TraceTypeQuery1" true 0 "None"))
  (if _returnvalue
    (bind _output_get (Variables|/Game/ThirdPerson/Blueprints/BP_ThirdPersonCharacter.BP_ThirdPersonCharacter_C|SetPreviewLocation _asbp_third_person_character (.Location (Collision|BreakHitResult _outhit))))
    (Utilities|IsValid (Variables|/Game/ThirdPerson/Blueprints/BP_ThirdPersonCharacter.BP_ThirdPersonCharacter_C|GetPreviewObj _asbp_third_person_character)
      (:Is%20Valid
        (Components|StaticMesh|SetStaticMesh (Variables|/Game/ThirdPerson/Blueprints/BP_ThirdPersonCharacter.BP_ThirdPersonCharacter_C|GetPreviewObj _asbp_third_person_character) (Variables|/Game/ThirdPerson/Blueprints/BP_ThirdPersonCharacter.BP_ThirdPersonCharacter_C|GetswitchMesh _asbp_third_person_character))
        (Transformation|SetWorldTransform (Variables|/Game/ThirdPerson/Blueprints/BP_ThirdPersonCharacter.BP_ThirdPersonCharacter_C|GetPreviewObj _asbp_third_person_character) (Math|Transform|MakeTransform (- _output_get "50.000000,50.000000,0.000000")) false false)))))

(event Input|KeyboardEvents|B
  (params (Key :type Key%20Structure :default "None"))
  (bind _returnvalue (Game|GetPlayerController 0))
  ;[1 1 1] shop
  (:Pressed
    (bind _returnvalue_2 (UserInterface|CreateWidget "/Game/Blueprints/UWBP_Shop.UWBP_Shop_C"))
    (Variables|Default|SetShopWidget _returnvalue_2)
    (UserInterface|Viewport|AddtoViewport _returnvalue_2 0)
    (Input|SetInputModeUIOnly _returnvalue 0 "DoNotLock" false)
    (Variables|/Script/Engine.PlayerController|SetbShowMouseCursor _returnvalue true)))

(event Input|KeyboardEvents|Tab
  (params (Key :type Key%20Structure :default "None"))
  (bind _returnvalue (Game|GetPlayerController 0))
  ;[1 1 1] menu
  (:Pressed
    (bind _asbp_third_person_character (Utilities|Casting|CastToBP_ThirdPersonCharacter (Game|GetPlayerCharacter 0)))
    (bind _returnvalue_2 (UserInterface|CreateWidget "/Game/Blueprints/uw_menu.uw_menu_C"))
    (Variables|/Game/ThirdPerson/Blueprints/BP_ThirdPersonCharacter.BP_ThirdPersonCharacter_C|Setwidget _asbp_third_person_character _returnvalue_2)
    (UserInterface|Viewport|AddtoViewport _returnvalue_2 0)
    (Input|SetInputModeUIOnly _returnvalue 0 "DoNotLock" false)
    (Variables|/Script/Engine.PlayerController|SetbShowMouseCursor _returnvalue true)))

(event Input|KeyboardEvents|E
  (params (Key :type Key%20Structure :default "None"))
  ;[1 1 1] spawning riht object
  (:Pressed
    (bind _asbp_third_person_character (Utilities|Casting|CastToBP_ThirdPersonCharacter (Game|GetPlayerCharacter 0)))
    (if (== (Variables|/Game/ThirdPerson/Blueprints/BP_ThirdPersonCharacter.BP_ThirdPersonCharacter_C|Getobjectindex _asbp_third_person_character) 0)
      (bind _returnvalue (Game|SpawnActorfromClass "/Game/Blueprints/bp_cube.bp_cube_C" (Math|Transform|MakeTransform (+ (Variables|/Game/ThirdPerson/Blueprints/BP_ThirdPersonCharacter.BP_ThirdPersonCharacter_C|GetPreviewLocation _asbp_third_person_character) "0.000000,0.000000,50.000000")) "Undefined" "MultiplyWithRoot" 0 0))
      (Utilities|Array|Add (Variables|/Game/ThirdPerson/Blueprints/BP_ThirdPersonCharacter.BP_ThirdPersonCharacter_C|Getthings%20to%20save _asbp_third_person_character) _returnvalue)
      (elif (== (Variables|/Game/ThirdPerson/Blueprints/BP_ThirdPersonCharacter.BP_ThirdPersonCharacter_C|Getobjectindex _asbp_third_person_character) 1)
        (bind _returnvalue_2 (Game|SpawnActorfromClass "/Game/Blueprints/bp_cyl.bp_cyl_C" (Math|Transform|MakeTransform (+ (Variables|/Game/ThirdPerson/Blueprints/BP_ThirdPersonCharacter.BP_ThirdPersonCharacter_C|GetPreviewLocation _asbp_third_person_character) "-50.000000,-50.000000,50.000000")) "Undefined" "MultiplyWithRoot" 0 0))
        (Utilities|Array|Add (Variables|/Game/ThirdPerson/Blueprints/BP_ThirdPersonCharacter.BP_ThirdPersonCharacter_C|Getthings%20to%20save _asbp_third_person_character) _returnvalue_2)
        (else
          (bind _returnvalue_3 (Game|SpawnActorfromClass "/Game/Blueprints/BP_ramp.BP_ramp_C" (Math|Transform|MakeTransform (+ (Variables|/Game/ThirdPerson/Blueprints/BP_ThirdPersonCharacter.BP_ThirdPersonCharacter_C|GetPreviewLocation _asbp_third_person_character) "-70.000000,-70.000000,-70.000000")) "Undefined" "MultiplyWithRoot" 0 0))
          (Utilities|Array|Add (Variables|/Game/ThirdPerson/Blueprints/BP_ThirdPersonCharacter.BP_ThirdPersonCharacter_C|Getthings%20to%20save _asbp_third_person_character) _returnvalue_3))))
    (Variables|/Game/ThirdPerson/Blueprints/BP_ThirdPersonCharacter.BP_ThirdPersonCharacter_C|Setbuild%20mode _asbp_third_person_character false)))

(fn PreviewLoop)